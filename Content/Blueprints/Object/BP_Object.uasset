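; BP_Object is an actor that bobs up and down while spinning continuously around its yaw axis.
; Each Tick, ZObjectMove flips the direction between the starting height and about 50 units above it, printing UP or DOWN for debugging.
; Tick then applies fixed per-frame height and yaw steps without delta time, so speed depends on frame rate.
; The downward reversal relies on exact equality with the starting Z.
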(event `self.ReceiveBeginPlay`
  (bind (_returnvalue_x _returnvalue_y _returnvalue_z) (`KismetMathLibrary.BreakVector` (`self.K2_GetActorLocation`)))
  (bind _output_get (set `self.Default Z Location` _returnvalue_z))
  (set `self.New Z location` _output_get)
  (set `self.Up` true))

(event `self.ReceiveTick`
  (params (DeltaSeconds :type "Float (single-precision)"))
  (bind (_returnvalue_roll _returnvalue_pitch _returnvalue_yaw) (`KismetMathLibrary.BreakRotator` (`self.K2_GetActorRotation`)))
  (bind (_returnvalue_x _returnvalue_y) (`KismetMathLibrary.BreakVector` (`self.K2_GetActorLocation`)))
  (`self.Z object move`)
  (bind _output_get (set `self.New Z location` (+ (`self.New Z location`) (`self.Z indentation`))))
  (`self.K2_SetActorLocationAndRotation` (`KismetMathLibrary.MakeVector` _returnvalue_x _returnvalue_y _output_get) (`KismetMathLibrary.MakeRotator` _returnvalue_roll _returnvalue_pitch (+ _returnvalue_yaw 2.0))))

(event `Z object move`
  (bind (_returnvalue_x _returnvalue_y _returnvalue_z) (`KismetMathLibrary.BreakVector` (`self.K2_GetActorLocation`)))
  (bind (_returnvalue_x_2 _returnvalue_y_2 _returnvalue_z_2) (`KismetMathLibrary.BreakVector` (`self.K2_GetActorLocation`)))
  (if (`self.Up`)
    (if (> _returnvalue_z (+ (`self.Default Z Location`) 50.0))
      (set `self.Z indentation` -1.0)
      (set `self.Up` false)
      (elif (`self.Up`)
        (set `self.Z indentation` 1.0)
        (`KismetSystemLibrary.PrintString` "UP" true true (struct :`G` 1.0 :`B` 0.121223 :`A` 1.0))))
    (elif (== _returnvalue_z_2 (`self.Default Z Location`))
      (set `self.Z indentation` 1.0)
      (set `self.Up` true)
      (else
        (set `self.Z indentation` -1.0)
        (`KismetSystemLibrary.PrintString` "DOWN" true true (struct :`G` 1.0 :`B` 0.121223 :`A` 1.0))))))

(fn `UserConstructionScript`)