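; BP_EnemyFollow is an enemy actor that homes in on the player character.
; Each Tick moves the static mesh along the normalized direction to the player, scaled by Speed and DeltaSeconds, and rotates it to face that direction.
; The player pawn's distance drives a clamped color lerp from red when near to white when far, sent to Niagara with the parameter name set to None.
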(event `self.ReceiveTick`
  (params (DeltaSeconds :type "Float (single-precision)"))
  (bind _returnvalue (`KismetMathLibrary.Normal` (- (`self.K2_GetActorLocation` (`GameplayStatics.GetPlayerCharacter` 0)) (`self.K2_GetActorLocation`))))
  (`SceneComponent.K2_SetWorldLocationAndRotation` (`self.StaticMesh`) (+ (* DeltaSeconds (`self.Speed`) _returnvalue) (`self.K2_GetActorLocation`)) (`KismetMathLibrary.MakeRotFromX` _returnvalue) false false)
  (`FXSystemComponent.SetColorParameter` (`self.Niagara`) "None" (`KismetMathLibrary.LinearColorLerp` (struct :`R` 0.682292 :`G` 0.110162 :`B` 0.110162 :`A` 1.0) (struct :`R` 1.0 :`G` 1.0 :`B` 1.0 :`A` 1.0) (`KismetMathLibrary.MapRangeClamped` (`self.GetDistanceTo` (`GameplayStatics.GetPlayerPawn` 0) null) 150.0 600.0 0.0 1.0))))

(fn `UserConstructionScript`)