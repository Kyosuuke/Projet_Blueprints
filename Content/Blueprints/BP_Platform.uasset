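; BP_Platform is a falling platform that drops after the player touches it and later returns to its original place.
; BeginPlay caches the static mesh's world location and rotation.
; A Hit from player character 0 waits briefly, enables physics simulation on the mesh, then after another delay disables it and restores the cached transform.
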(event `self.ReceiveHit`
  (params (MyComp :type "PrimitiveComponent Object Reference") (Other :type "Actor Object Reference") (OtherComp :type "PrimitiveComponent Object Reference") (bSelfMoved :type Boolean) (HitLocation :type "Vector Structure") (HitNormal :type "Vector Structure") (NormalImpulse :type "Vector Structure") (Hit :type "HitResult Structure (by ref)"))
  (bind _staticmesh (`self.StaticMesh`))
  (if (== Other (`GameplayStatics.GetPlayerCharacter` 0))
    (`KismetSystemLibrary.Delay` 2.0)
    (`PrimitiveComponent.SetSimulatePhysics` _staticmesh true)
    (`KismetSystemLibrary.Delay` 3.0)
    (`PrimitiveComponent.SetSimulatePhysics` _staticmesh false)
    (`SceneComponent.K2_SetWorldTransform` _staticmesh (`KismetMathLibrary.MakeTransform` (`self.Default location`) (`self.Default rotation`)) false false)))

(event `self.ReceiveBeginPlay`
  (bind _staticmesh (`self.StaticMesh`))
  (set `self.Default location` (`SceneComponent.K2_GetComponentLocation` _staticmesh))
  (set `self.Default rotation` (`SceneComponent.K2_GetComponentRotation` _staticmesh)))

(fn `UserConstructionScript`)