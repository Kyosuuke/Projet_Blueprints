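; BP_Shooting is an actor that periodically fires projectiles at the player.
; A looping timer started on BeginPlay checks whether the player character is within range.
; If so, it spawns a Bp_Projectile slightly above itself and pushes its Sphere component with an impulse along the direction to the player, scaled by a Force variable.
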(event `self.ReceiveBeginPlay`
  (`KismetSystemLibrary.K2_SetTimerDelegate` (delegate `Shoot`) 2.0 true))

(event `Shoot`
  (bind _returnvalue (`GameplayStatics.GetPlayerCharacter` 0))
  (if (<= (`self.GetDistanceTo` _returnvalue) 500.0)
    (bind _returnvalue_2 (`|SpawnActorFromClass` "/Game/TowerDefense/TD_Blueprints/Bp_Fabien/Bp_Projectile.Bp_Projectile_C" (`KismetMathLibrary.Conv_VectorToTransform` (+ (`self.K2_GetActorLocation`) (0.0 0.0 65.0))) "Undefined" "MultiplyWithRoot" null null))
    (`PrimitiveComponent.AddImpulse` (`/Game/TowerDefense/TD_Blueprints/Bp_Fabien/Bp_Projectile.Sphere` _returnvalue_2) (* (`KismetMathLibrary.GetDirectionUnitVector` (`self.K2_GetActorLocation`) (`self.K2_GetActorLocation` _returnvalue)) (`self.Force`)) "None" false)))

(fn `UserConstructionScript`)