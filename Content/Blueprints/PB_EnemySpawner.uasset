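; An enemy spawner actor that releases enemies in endless rounds, each two enemies larger than the last.
; A looping timer fires SpawnEvent, which plays a Niagara effect around spawning an Enemy slightly above the actor and decrements the round's counter.
; Tick detects an exhausted counter, grows the next round and restarts the timer at triple the interval.
; The first firing of a new round only restores the normal interval.
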(event `Timer Reset`
  (`KismetSystemLibrary.K2_SetTimerDelegate` (delegate `SpawnEvent`) (`self.new Spawn Time`) true :!label _label))

(event `self.ReceiveBeginPlay`
  ;[0 0 0] Initialize the variable
  (set `self.Enemy Actual Number` (`self.Enemy Number (First Round)`))
  (set `self.new Spawn Time` (`self.Spawn Time`))
  (goto _label))

(event `SpawnEvent`
  (bind (_returnvalue_x _returnvalue_y _returnvalue_z) (`KismetMathLibrary.BreakVector` (`self.K2_GetActorLocation`)))
  (if (`self.NewRound`)
    ;[0 0 0] Reset the spawn enemies timer after the start of new round
    (set `self.new Spawn Time` (`self.Spawn Time`))
    (set `self.NewRound` false)
    (`self.Timer Reset`)
    (else
      (`ActorComponent.Activate` (`self.Niagara`) false)
      (`KismetSystemLibrary.Delay` 1.0)
      ;[0 0 0] Create the "Enemy" variable
      (`|SpawnActorFromClass` (`self.Enemy`) (`KismetMathLibrary.Conv_VectorToTransform` (`KismetMathLibrary.MakeVector` _returnvalue_x _returnvalue_y (+ _returnvalue_z 80.0))) "Undefined" "MultiplyWithRoot" null null)
      ;[0 0 0] Substract the number of enemies to spawn
      (set `self.Enemy Actual Number` (- (`self.Enemy Actual Number`) 1))
      (`KismetSystemLibrary.Delay` 2.0)
      (`ActorComponent.Deactivate` (`self.Niagara`)))))

(event `self.ReceiveTick`
  (params (DeltaSeconds :type "Float (single-precision)"))
  (bind _spawn_time (`self.Spawn Time`))
  ;[0 0 0] If all enemies round have spawn
  (if (<= (`self.Enemy Actual Number`) 0)
    ;[0 0 0] Up the number of enemies how going to spawn
    (set `self.Enemy Number (First Round)` (+ (`self.Enemy Number (First Round)`) 2))
    (set `self.Enemy Actual Number` (`self.Enemy Number (First Round)`))
    ;[0 0 0] The next spawn will start later
    (set `self.new Spawn Time` (+ _spawn_time (* _spawn_time 2.0)))
    (`KismetSystemLibrary.PrintString` "New Round" true true (struct :`R` 0.453125 :`B` 0.045563 :`A` 1.0))
    (set `self.NewRound` true)
    (`self.Timer Reset`)))

(fn `UserConstructionScript`)