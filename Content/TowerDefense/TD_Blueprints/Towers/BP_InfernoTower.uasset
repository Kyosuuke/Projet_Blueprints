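; Inferno tower for a tower defense game that burns one enemy with a laser whose damage ramps up over time.
; A sphere overlap tracks enemies in range, and a one-second timer prunes dead ones and picks a target when none is valid.
; Tick aims the Niagara beam and applies per-frame damage scaled by active time, resetting on the kill.
; Leaving range does not clear the current target.
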(event `self.ReceiveBeginPlay`
  ;[1 1 1] Set ray to false
  (`ActorComponent.SetActive` (`self.P_Laser_03`) false false)
  (`KismetSystemLibrary.K2_SetTimerDelegate` (delegate `Check Targets`) 1.0 true))

(event `Check Targets`
  (bind _enemies_in_range (`self.Enemies in range`))
  ;[1 1 1] Set new target
  (for _array_element _enemies_in_range
    (if (<= (`/Game/TowerDefense/TD_Blueprints/Enemies/BP_Enemy.Health` _array_element) 0.0)
      (`KismetArrayLibrary.Array_RemoveItem` _enemies_in_range)
      (else
        (`self.Target`
          (:`then`)
          (:`else`
            (set `self.Target` _array_element)))))))

(event `self.Sphere.OnComponentBeginOverlap`
  (params (OverlappedComponent :type "PrimitiveComponent Object Reference") (OtherActor :type "Actor Object Reference") (OtherComp :type "PrimitiveComponent Object Reference") (OtherBodyIndex :type Integer) (bFromSweep :type Boolean) (SweepResult :type "HitResult Structure (by ref)"))
  ;[1 1 1] Adds Enemy to array of enemies
  (if (`self.ActorHasTag` OtherActor "Enemy")
    (bind _asbp_enemy (cast `/Game/TowerDefense/TD_Blueprints/Enemies/BP_Enemy` OtherActor))
    (`KismetArrayLibrary.Array_AddUnique` (`self.Enemies in range`) _asbp_enemy)))

(event `self.Sphere.OnComponentEndOverlap`
  (params (OverlappedComponent :type "PrimitiveComponent Object Reference") (OtherActor :type "Actor Object Reference") (OtherComp :type "PrimitiveComponent Object Reference") (OtherBodyIndex :type Integer))
  ;[1 1 1] Removes enemies that get out of range
  (if (`self.ActorHasTag` OtherActor "Enemy")
    (bind _asbp_enemy (cast `/Game/TowerDefense/TD_Blueprints/Enemies/BP_Enemy` OtherActor))
    (`KismetArrayLibrary.Array_RemoveItem` (`self.Enemies in range`) _asbp_enemy)))

(event `self.ReceiveTick`
  (params (DeltaSeconds :type "Float (single-precision)"))
  (bind _p_laser_03 (`self.P_Laser_03`))
  ;[1 1 1] Set niagara active and to target
  (bind _target (`self.Target`)
    (:`then`
      (if (`ActorComponent.IsActive` _p_laser_03)
        (`FXSystemComponent.SetVectorParameter` _p_laser_03 "User.End" (`self.K2_GetActorLocation` _target))
        (bind _output_get (set `self.TimeActivated` (+ (`self.TimeActivated`) DeltaSeconds)))
        (`GameplayStatics.ApplyDamage` (`self.Target`) (* _output_get (`self.Base Damage`)))
        (if (<= (`/Game/TowerDefense/TD_Blueprints/Enemies/BP_Enemy.Health` (`self.Target`)) 0.0)
          (`ActorComponent.SetActive` (`self.P_Laser_03`) false false)
          (set `self.TimeActivated` 0.0))
        (else
          (`ActorComponent.SetActive` _p_laser_03 true false))))
    (:`else`)))

(fn `UserConstructionScript`)