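; Tower defense projectile actor that costs a life when it hits the player, and destroys itself one second after spawning.
; When its sphere overlaps player character 0, it decrements Life on the Bp_Tower found by GetActorOfClass, so the counter lives on the tower.
; If that Life is already zero at the overlap, it opens the Fabien level instead, intended as a restart.
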(event `self.ReceiveBeginPlay`
  ;[0 0 0] Destroy after 1 sec
  (`KismetSystemLibrary.Delay` 1.0)
  (`self.K2_DestroyActor`))

(event `self.Sphere1.OnComponentBeginOverlap`
  (params (OverlappedComponent :type "PrimitiveComponent Object Reference") (OtherActor :type "Actor Object Reference") (OtherComp :type "PrimitiveComponent Object Reference") (OtherBodyIndex :type Integer) (bFromSweep :type Boolean) (SweepResult :type "HitResult Structure (by ref)"))
  ;[0 0 0] Decrement Life and restart if under 0
  (if (== OtherActor (`GameplayStatics.GetPlayerCharacter` 0))
    (bind _returnvalue (`GameplayStatics.GetActorOfClass` "/Game/TowerDefense/TD_Blueprints/Bp_Tower.Bp_Tower_C"))
    (bind _life (`/Game/TowerDefense/TD_Blueprints/Bp_Tower.Life` _returnvalue))
    (if (== _life 0)
      (`GameplayStatics.OpenLevelBySoftObjectPtr` "/Game/TowerDefense/TD_Maps/Fabien.Fabien")
      (else
        (`/Engine/EditorBlueprintResources/StandardMacros.DecrementInt` _life)))))

(fn `UserConstructionScript`)