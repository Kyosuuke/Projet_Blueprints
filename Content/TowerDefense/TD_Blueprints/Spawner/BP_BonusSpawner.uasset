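; BP_BonusSpawner is a tower defense actor that spawns a single bonus pickup above its platform.
; On BeginPlay it calls SpawnBonus, which waits TimerSpawn plus a random extra delay, then randomly spawns either a HealthPack or a SpeedPack slightly above the actor's location.
; The graph contains no loop or respawn call, so any repeat spawn depends on SpawnBonus being triggered from elsewhere.
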(event `self.ReceiveBeginPlay`
  (`self.Spawn Bonus`))

(event `Spawn Bonus`
  (bind (_returnvalue_x _returnvalue_y _returnvalue_z) (`KismetMathLibrary.BreakVector` (`self.K2_GetActorLocation`)))
  (bind _returnvalue (`KismetMathLibrary.MakeVector` _returnvalue_x _returnvalue_y (+ _returnvalue_z 80.0)))
  (`KismetSystemLibrary.Delay` (+ (`self.Timer Spawn`) (`KismetMathLibrary.RandomFloatInRange` 1.0 (`self.Timer Spawn`))))
  (if (`KismetMathLibrary.RandomBool`)
    ;[0 0 0] Spawn Health pack
    (`|SpawnActorFromClass` (`self.HealthPack`) (`KismetMathLibrary.Conv_VectorToTransform` _returnvalue) "Undefined" "MultiplyWithRoot" null null)
    (else
      ;[0 0 0] Spawn Speed pack
      (`|SpawnActorFromClass` (`self.SpeedPack`) (`KismetMathLibrary.Conv_VectorToTransform` _returnvalue) "Undefined" "MultiplyWithRoot" null null))))

(fn `UserConstructionScript`)