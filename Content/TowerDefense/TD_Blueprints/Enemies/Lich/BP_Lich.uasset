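; Lich enemy for the tower defense game that attacks the nearest tower and heals wounded allies.
; An overlap sphere tracks nearby enemies, and a one-second timer targets one below a health threshold.
; A faster movement timer halts the Lich while that target is low, otherwise moves it towards the tower.
; HealAlly (Goblins only, capped), CastHealSpell and DealDamage are not called within this Blueprint; Tick handles death.
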(event `self.ReceiveBeginPlay`
  ;[1 1 1] On Begin
  (`parent.ReceiveBeginPlay`)
  (`ActorComponent.SetActive` (`self.Niagara`) false false)
  (set `self.Health` (`self.MaxHealth`))
  (`self.UpdateHealthBar` (`WidgetComponent.GetUserWidgetObject` (`self.HealthBar`)) (`self.MaxHealth`))
  (`self.FindTargetTower`)
  (`KismetSystemLibrary.Delay` 2.0)
  (`KismetSystemLibrary.K2_SetTimerDelegate` (delegate `Movement`) 0.1 true)
  ;[1 1 1] Checks for Targets to heal
  (`KismetSystemLibrary.K2_SetTimerDelegate` (delegate `ApplyTarget`) 1.0 true))

(event `ApplyTarget`
  ;[1 1 1] Checks for Targets to heal
  (`self.CheckForTargetAlly`)
  (`ActorComponent.Deactivate` (`self.Niagara`)))

(event `self.ReceiveAnyDamage`
  (params (Damage :type "Float (single-precision)") (DamageType :type "DamageType Object Reference") (InstigatedBy :type "Controller Object Reference") (DamageCauser :type "Actor Object Reference"))
  ;[1 1 1] Update Life
  (`self.UpdateLife` Damage)
  (`self.UpdateHealthBar` (`WidgetComponent.GetUserWidgetObject` (`self.HealthBar`)) (`self.MaxHealth`))
  (`ActorComponent.Activate` (`self.Niagara`) false))

(event `Movement`
  ;[1 1 1] Movements to Tower
  (bind _healstate (`self.CheckHealingState`))
  (if _healstate
    (`MovementComponent.StopMovementImmediately` (`self.CharacterMovement`))
    (set `self.IsAttacking` false)
    (else
      (bind _tower (`self.Tower`)
        (:`then`
          (`|AIMoveTo` self (0.0 0.0 0.0) _tower 300.0
            (:`OnSuccess`
              (set `self.IsAttacking` true))))
        (:`else`
          (`self.FindTargetTower`))))))

(event `self.Sphere.OnComponentBeginOverlap`
  (params (OverlappedComponent :type "PrimitiveComponent Object Reference") (OtherActor :type "Actor Object Reference") (OtherComp :type "PrimitiveComponent Object Reference") (OtherBodyIndex :type Integer) (bFromSweep :type Boolean) (SweepResult :type "HitResult Structure (by ref)"))
  ;[1 1 1] Adds Ally to list
  (if (`self.ActorHasTag` OtherActor "Enemy")
    (if (not (== OtherActor self))
      (bind _asbp_enemy (cast `/Game/TowerDefense/TD_Blueprints/Enemies/BP_Enemy` OtherActor))
      (`KismetArrayLibrary.Array_AddUnique` (`self.Allies`) _asbp_enemy))))

(event `self.Sphere.OnComponentEndOverlap`
  (params (OverlappedComponent :type "PrimitiveComponent Object Reference") (OtherActor :type "Actor Object Reference") (OtherComp :type "PrimitiveComponent Object Reference") (OtherBodyIndex :type Integer))
  ;[1 1 1] Remove Ally from list
  (if (`self.ActorHasTag` OtherActor "Enemy")
    (bind _asbp_enemy (cast `/Game/TowerDefense/TD_Blueprints/Enemies/BP_Enemy` OtherActor))
    (`KismetArrayLibrary.Array_RemoveItem` (`self.Allies`) _asbp_enemy)))

(event `self.ReceiveTick`
  (params (DeltaSeconds :type "Float (single-precision)"))
  ;[1 1 1] Check if dead
  (`parent.ReceiveTick` DeltaSeconds)
  (if (<= (`self.Health`) 0.0)
    (set `self.IsDead` true)
    (`ActorComponent.SetActive` (`self.Niagara`) false false)
    (`self.DetachFromControllerPendingDestroy`)
    (`KismetSystemLibrary.Delay` 2.0)
    (`self.K2_DestroyActor`)))

(fn `Cast HealSpell`
  (bind _healspell (`self.HealSpell`))
  (`SceneComponent.K2_SetWorldLocation` _healspell (- (`self.K2_GetActorLocation` (`self.Target`)) (0.0 0.0 60.0)) false true)
  (`ActorComponent.Activate` _healspell false))

(fn `CheckForTargetAlly`
  (for _array_element (`self.Allies`)
    (`/Engine/EditorBlueprintResources/StandardMacros.IsValid` _array_element
      (:`Is Valid`
        (if (`/Game/TowerDefense/TD_Blueprints/Enemies/BP_Enemy.IsDead` _array_element)
          (`KismetArrayLibrary.Array_RemoveItem` (`self.Allies`))
          (elif (< (`/Game/TowerDefense/TD_Blueprints/Enemies/BP_Enemy.Health` _array_element) (`self.TargetHealth`))
            (set `self.Target` _array_element)))))))

(fn `CheckHealingState`
  (returns (HealState :type Boolean))
  (bind _target (`self.Target`)
    (:`then`
      (if (`/Game/TowerDefense/TD_Blueprints/Enemies/BP_Enemy.IsDead` _target)
        _
        (elif (<= (`/Game/TowerDefense/TD_Blueprints/Enemies/BP_Enemy.Health` _target) 250.0)
          (bind _output_get (set `self.IsHealingAlly` true))
          (return _output_get)
          (else
            _))))
    (:`else`
      _))
  (bind _output_get_2 (set `self.IsHealingAlly` false))
  (return _output_get_2))

(fn `DealDamage`
  (params (Damage :type "Float (double-precision)"))
  (`GameplayStatics.ApplyDamage` (`self.Tower`) Damage))

(fn `FindTargetTower`
  (set `self.TowerDist` 2000000.0)
  (bind _outactors (`GameplayStatics.GetAllActorsWithTag` "Tower"))
  (for _array_element _outactors
    (`/Engine/EditorBlueprintResources/StandardMacros.IsValid` _array_element
      (:`Is Valid`
        (bind _returnvalue (`KismetMathLibrary.Vector_Distance` (`self.K2_GetActorLocation` _array_element) (`self.K2_GetActorLocation`)))
        (if (< _returnvalue (`self.TowerDist`))
          (set `self.Tower` _array_element)
          (set `self.TowerDist` _returnvalue)))))
  (return))

(fn `HealAlly`
  (bind _target (`self.Target`))
  (bind _health (`/Game/TowerDefense/TD_Blueprints/Enemies/BP_Enemy.Health` (`self.Target`)))
  (bind _returnvalue (+ _health (`self.HealAmount`)))
  (if (not (<= _health 0.0))
    (bind _asbp_goblin (cast `/Game/TowerDefense/TD_Blueprints/Enemies/Goblin/BP_Goblin` (`self.Target`)))
    (bind _goblinhealth (`/Game/TowerDefense/TD_Blueprints/Enemies/Goblin/BP_Goblin.GoblinHealth` _asbp_goblin))
    (if (> _returnvalue _goblinhealth)
      (set `/Game/TowerDefense/TD_Blueprints/Enemies/BP_Enemy.Health` _goblinhealth _target)
      (else
        (set `/Game/TowerDefense/TD_Blueprints/Enemies/BP_Enemy.Health` _returnvalue _target)))))

(fn `Move to tower`)

(fn `UpdateHealthBar`
  (params (Widget :type "Widget Object Reference") (Health :type "Float (double-precision)"))
  (`parent.UpdateHealthBar` Widget Health))

(fn `UpdateLife`
  (params (Damage1 :type "Float (double-precision)"))
  (`parent.UpdateLife` Damage1))

(fn `UserConstructionScript`
  (`parent.UserConstructionScript`))