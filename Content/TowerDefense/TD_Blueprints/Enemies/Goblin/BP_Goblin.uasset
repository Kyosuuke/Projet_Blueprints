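; Goblin enemy for the tower defense game, a child Blueprint that passes construction, life and health bar updates through to its parent.
; BeginPlay seeds Health from GoblinHealth, fills the health bar widget and switches off the Niagara effect.
; Damage calls UpdateLife, refreshes the bar from GoblinHealth and activates the effect.
; Tick polls Health, and at zero flags death, stops the effect, detaches the controller and destroys the actor after a delay.
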(event `self.ReceiveBeginPlay`
  ;[1 1 1] Setting Health
  (`parent.ReceiveBeginPlay`)
  (set `self.Health` (`self.GoblinHealth`))
  (`self.UpdateHealthBar` (`WidgetComponent.GetUserWidgetObject` (`self.HealthBar`)) (`self.GoblinHealth`))
  (`ActorComponent.SetActive` (`self.Niagara`) false false))

(event `self.ReceiveTick`
  (params (DeltaSeconds :type "Float (single-precision)"))
  ;[1 1 1] Check if dead
  (if (<= (`self.Health`) 0.0)
    (set `self.IsDead` true)
    (`ActorComponent.SetActive` (`self.Niagara`) false false)
    (`self.DetachFromControllerPendingDestroy`)
    (`KismetSystemLibrary.Delay` 2.0)
    (`self.K2_DestroyActor`)))

(event `self.ReceiveAnyDamage`
  (params (Damage :type "Float (single-precision)") (DamageType :type "DamageType Object Reference") (InstigatedBy :type "Controller Object Reference") (DamageCauser :type "Actor Object Reference"))
  ;[1 1 1] Apply damage
  (`self.UpdateLife` Damage)
  (`self.UpdateHealthBar` (`WidgetComponent.GetUserWidgetObject` (`self.HealthBar`)) (`self.GoblinHealth`))
  (`ActorComponent.Activate` (`self.Niagara`) false))

(fn `UpdateHealthBar`
  (params (Widget :type "Widget Object Reference") (Health :type "Float (double-precision)"))
  (`parent.UpdateHealthBar` Widget Health))

(fn `UpdateLife`
  (params (Damage1 :type "Float (double-precision)"))
  (`parent.UpdateLife` Damage1))

(fn `UserConstructionScript`
  (`parent.UserConstructionScript`))