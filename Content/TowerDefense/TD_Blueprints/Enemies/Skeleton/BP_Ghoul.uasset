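; BP_Ghoul is a skeleton-category tower defense enemy that chases the first-person player and dies when its health runs out.
; A looping timer drives AI movement toward the player, stopping in range and resuming once the player leaves attack range.
; Damage and health bar updates defer to the parent class, while Tick detects death, detaches the controller and destroys the actor after a delay.
; DealDamage applies damage to the player but is not called here.
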(event `self.ReceiveBeginPlay`
  ;[1 1 1] On Begin
  (`parent.ReceiveBeginPlay`)
  (bind _returnvalue (`GameplayStatics.GetActorOfClass` "/Game/TowerDefense/TD_Blueprints/BP_FirstPersonCharacter.BP_FirstPersonCharacter_C"))
  (set `self.Player` _returnvalue)
  (set `self.Health` (`self.GhoulHealth`))
  (`self.UpdateHealthBar` (`WidgetComponent.GetUserWidgetObject` (`self.HealthBar`)) (`self.GhoulHealth`))
  (`KismetSystemLibrary.K2_SetTimerDelegate` (delegate `Movements`) 0.1 true))

(event `Movements`
  ;[1 1 1] Ghoul Movements
  (`self.CheckInRange`)
  (if (`self.InRange`)
    (`MovementComponent.StopMovementImmediately` (`self.CharacterMovement`))
    (else
      (`|AIMoveTo` self (0.0 0.0 0.0) (`self.Player`) 25.0
        (:`OnSuccess`
          (set `self.InRange` true))))))

(event `self.ReceiveTick`
  (params (DeltaSeconds :type "Float (single-precision)"))
  ;[1 1 1] Check If Dead
  (`parent.ReceiveTick` DeltaSeconds)
  (if (<= (`self.Health`) 0.0)
    (set `self.IsDead` true)
    (`self.DetachFromControllerPendingDestroy`)
    (`KismetSystemLibrary.Delay` 2.0)
    (`self.K2_DestroyActor`)))

(event `self.ReceiveAnyDamage`
  (params (Damage :type "Float (single-precision)") (DamageType :type "DamageType Object Reference") (InstigatedBy :type "Controller Object Reference") (DamageCauser :type "Actor Object Reference"))
  ;[1 1 1] Update Life
  (`self.UpdateLife` Damage)
  (`self.UpdateHealthBar` (`WidgetComponent.GetUserWidgetObject` (`self.HealthBar`)) (`self.GhoulHealth`)))

(fn `CheckInRange`
  (if (>= (`self.GetDistanceTo` (`self.Player`) self) (`self.AttackRange`))
    (set `self.InRange` false)))

(fn `DealDamage`
  (params (Damage :type "Float (double-precision)"))
  (`GameplayStatics.ApplyDamage` (`self.Player`) Damage))

(fn `Move to Player`)

(fn `UpdateHealthBar`
  (params (Widget :type "Widget Object Reference") (Health :type "Float (double-precision)"))
  (`parent.UpdateHealthBar` Widget Health))

(fn `UpdateLife`
  (params (Damage1 :type "Float (double-precision)"))
  (`parent.UpdateLife` Damage1))

(fn `UserConstructionScript`
  (`parent.UserConstructionScript`))