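; Goblin enemy for the tower defense game that takes damage, shows a health bar and dies at zero health.
; BeginPlay fills health, and AnyDamage calls the parent's life and health bar updates, passing MaxHealth to the bar.
; Tick polls health, then flags death, detaches the controller and destroys the actor after a short delay.
; An Inferno Tower damage-causer check leads to no action.
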(event `self.ReceiveBeginPlay`
  (bind _maxhealth (`self.MaxHealth`))
  ;[1 1 1] Setting Health
  (`parent.ReceiveBeginPlay`)
  (set `self.Health` _maxhealth)
  (`self.UpdateHealthBar` (`WidgetComponent.GetUserWidgetObject` (`self.WB_HealthBar`)) _maxhealth))

(event `self.ReceiveTick`
  (params (DeltaSeconds :type "Float (single-precision)"))
  ;[1 1 1] Check if dead
  (if (<= (`self.Health`) 0.0)
    (set `self.IsDead` true)
    (`self.DetachFromControllerPendingDestroy`)
    (`KismetSystemLibrary.Delay` 2.0)
    (`self.K2_DestroyActor`)))

(event `self.ReceiveAnyDamage`
  (params (Damage :type "Float (single-precision)") (DamageType :type "DamageType Object Reference") (InstigatedBy :type "Controller Object Reference") (DamageCauser :type "Actor Object Reference"))
  ;[1 1 1] Apply damage
  (`self.UpdateLife` Damage)
  (`self.UpdateHealthBar` (`WidgetComponent.GetUserWidgetObject` (`self.WB_HealthBar`)) (`self.MaxHealth`))
  (bind _returnvalue (`GameplayStatics.GetActorOfClass` "/Game/TowerDefense/TD_Blueprints/Towers/BP_InfernoTower.BP_InfernoTower_C"))
  (if (== DamageCauser _returnvalue)
    _))

(fn `UpdateHealthBar`
  (params (WB_HealthBar :type "Widget Object Reference") (HealthEnemy :type "Float (double-precision)"))
  (`parent.UpdateHealthBar` WB_HealthBar HealthEnemy)
  (return))

(fn `UpdateLife`
  (params (Damage1 :type "Float (double-precision)"))
  (`parent.UpdateLife` Damage1))

(fn `UserConstructionScript`
  (`parent.UserConstructionScript`))