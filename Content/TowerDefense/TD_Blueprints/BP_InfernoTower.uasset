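; Inferno tower for the tower defense game that aims a laser effect at an enemy; no damage logic is present.
; A sphere overlap replaces the in-range list with the entering "Enemy"-tagged actor, and end overlap removes it.
; Tick prunes invalid entries, picks a Target when none is valid, then activates the laser or moves its User.End parameter to the Target.
; Target is never cleared on leaving range, and the laser is only deactivated at BeginPlay.
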(event `self.ReceiveBeginPlay`
  ;[1 1 1] Set ray to false
  (`ActorComponent.SetActive` (`self.P_Laser_03`) false false))

(event `self.ReceiveTick`
  (params (DeltaSeconds :type "Float (single-precision)"))
  (bind _p_laser_03 (`self.P_Laser_03`))
  (bind _target (`self.Target`))
  (bind _enemies_in_range (`self.Enemies in range`))
  ;[1 1 1] Checks if all enemies are allive, if not remove them from list. Then checks if InfernoRay is actif, and if not activates it.
  (for _array_element _enemies_in_range
    (`/Engine/EditorBlueprintResources/StandardMacros.IsValid` _array_element
      (:`Is Valid`
        (`/Engine/EditorBlueprintResources/StandardMacros.IsValid` _target
          (:`Is Valid`
            (if (`ActorComponent.IsActive` _p_laser_03)
              (`FXSystemComponent.SetVectorParameter` _p_laser_03 "User.End" (`self.K2_GetActorLocation` _target))
              (else
                (`ActorComponent.SetActive` _p_laser_03 true false))))
          (:`Is Not Valid`
            (set `self.Target` _array_element))))
      (:`Is Not Valid`
        (`KismetArrayLibrary.Array_RemoveItem` _enemies_in_range _array_element)))))

(event `self.Sphere.OnComponentBeginOverlap`
  (params (OverlappedComponent :type "PrimitiveComponent Object Reference") (OtherActor :type "Actor Object Reference") (OtherComp :type "PrimitiveComponent Object Reference") (OtherBodyIndex :type Integer) (bFromSweep :type Boolean) (SweepResult :type "HitResult Structure (by ref)"))
  ;[1 1 1] Adds Enemy to array of actors
  (for _array_element (`Actor.Tags` OtherActor)
    (if (== _array_element "Enemy")
      (set `self.Enemies in range` (`|MakeArray` OtherActor)))))

(event `self.Sphere.OnComponentEndOverlap`
  (params (OverlappedComponent :type "PrimitiveComponent Object Reference") (OtherActor :type "Actor Object Reference") (OtherComp :type "PrimitiveComponent Object Reference") (OtherBodyIndex :type Integer))
  (bind _enemies_in_range (`self.Enemies in range`))
  ;[1 1 1] Removes enemies that get out of range
  (for _array_element _enemies_in_range
    (if (== _array_element OtherActor)
      (`KismetArrayLibrary.Array_RemoveItem` _enemies_in_range OtherActor))))

(fn `UserConstructionScript`)