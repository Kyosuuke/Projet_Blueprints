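; Magic staff weapon actor that the first-person character can attach to its mesh while nearby.
; The PlayerDetect overlap stores or clears the player reference, which gates the PickWeapon input.
; Each press flip-flops between snapping the static mesh to the GripPoint socket and detaching the actor.
; A custom event applies a fixed local rotation step, ignoring its DeltaSeconds input, and nothing in these graphs calls it.
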(event `InputAction|PickWeapon`
  (params (Key :type "Key Structure"))
  (bind _playerref (`self.PlayerRef`))
  (:`Pressed`
    (`/Engine/EditorBlueprintResources/StandardMacros.IsValid` _playerref
      (:`Is Valid`
        (`/Engine/EditorBlueprintResources/StandardMacros.FlipFlop`
          (:`A`
            (`SceneComponent.K2_AttachToComponent` (`self.StaticMesh`) (`Character.Mesh` _playerref) "GripPoint" "SnapToTarget" "SnapToTarget" "KeepWorld" true))
          (:`B`
            (`self.K2_DetachFromActor` "KeepWorld" "KeepWorld" "KeepWorld")))))))

(event `self.PlayerDetect.OnComponentBeginOverlap`
  (params (OverlappedComponent :type "PrimitiveComponent Object Reference") (OtherActor :type "Actor Object Reference") (OtherComp :type "PrimitiveComponent Object Reference") (OtherBodyIndex :type Integer) (bFromSweep :type Boolean) (SweepResult :type "HitResult Structure (by ref)"))
  (bind _asbp_first_person_character (cast `/Game/TowerDefense/TD_Blueprints/BP_FirstPersonCharacter` OtherActor))
  (set `self.PlayerRef` _asbp_first_person_character))

(event `self.PlayerDetect.OnComponentEndOverlap`
  (params (OverlappedComponent :type "PrimitiveComponent Object Reference") (OtherActor :type "Actor Object Reference") (OtherComp :type "PrimitiveComponent Object Reference") (OtherBodyIndex :type Integer))
  (cast `/Game/TowerDefense/TD_Blueprints/BP_FirstPersonCharacter` OtherActor)
  (set `self.PlayerRef` null))

(event `CustomEvent`
  (params (DeltaSeconds :type "Float (single-precision)"))
  (`self.K2_AddActorLocalRotation` (struct :`Yaw` 5.0 :`Roll` 30.0)))

(fn `UserConstructionScript`)