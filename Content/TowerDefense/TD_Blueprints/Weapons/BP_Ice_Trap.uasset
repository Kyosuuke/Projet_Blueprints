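; Ice trap for the tower defense game that damages and slows enemies walking into its box trigger.
; An overlapping BP_Enemy tagged "Enemy" sets off a particle effect and radial damage around the trap, and has its walk speed reduced with no restore.
; The trap removes the effect and itself after a short delay, with no guard against other enemies triggering it meanwhile.
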(event `self.Box.OnComponentBeginOverlap`
  (params (OverlappedComponent :type "PrimitiveComponent Object Reference") (OtherActor :type "Actor Object Reference") (OtherComp :type "PrimitiveComponent Object Reference") (OtherBodyIndex :type Integer) (bFromSweep :type Boolean) (SweepResult :type "HitResult Structure (by ref)"))
  (bind _returnvalue (`self.K2_GetActorLocation`))
  (bind _asbp_enemy (cast `/Game/TowerDefense/TD_Blueprints/Enemies/BP_Enemy` OtherActor))
  (if (`self.ActorHasTag` OtherActor "Enemy")
    (bind _returnvalue_2 (`NiagaraFunctionLibrary.SpawnSystemAtLocation` "/Game/Stylized_VFX_StPack/Particles/UPDATE_1_2/P_Cosmic_Projectile_02.P_Cosmic_Projectile_02" _returnvalue))
    (`GameplayStatics.ApplyRadialDamage` :`BaseDamage` 30.0 :`Origin` _returnvalue :`DamageRadius` 300.0 :`DamageCauser` null :`InstigatedByController` null)
    (bind _charactermovement (`Character.CharacterMovement` _asbp_enemy))
    (set `CharacterMovementComponent.MaxWalkSpeed` (/ (`MovementComponent.GetMaxSpeed` _charactermovement) 1.5) _charactermovement)
    (`KismetSystemLibrary.Delay` 3.0)
    (`ActorComponent.K2_DestroyComponent` _returnvalue_2)
    (`self.K2_DestroyActor`)))

(fn `UserConstructionScript`)