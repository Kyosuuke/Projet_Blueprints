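; BP_Rocket is a rocket projectile in the tower defense game's weapons set.
; On hitting a physics-simulating component, it adds a velocity-scaled impulse at its location, calls ApplyDamage with itself as causer, then destroys itself.
; Hits on non-simulating components have no scripted effect, and a short timer from BeginPlay destroys the rocket regardless.
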(event `self.ReceiveHit`
  (params (MyComp :type "PrimitiveComponent Object Reference") (Other :type "Actor Object Reference") (OtherComp :type "PrimitiveComponent Object Reference") (bSelfMoved :type Boolean) (HitLocation :type "Vector Structure") (HitNormal :type "Vector Structure") (NormalImpulse :type "Vector Structure") (Hit :type "HitResult Structure (by ref)"))
  (if (`SceneComponent.IsSimulatingPhysics` OtherComp "None")
    (`PrimitiveComponent.AddImpulseAtLocation` OtherComp (* (`self.GetVelocity`) 100.0) (`self.K2_GetActorLocation`) "None")
    (`GameplayStatics.ApplyDamage` null 3.0 null self)
    (`self.K2_DestroyActor`) ; Then destroy this projectile
  ))

(event `self.ReceiveBeginPlay`
  (`KismetSystemLibrary.Delay` 4.0)
  (`self.K2_DestroyActor`) ; Then destroy this projectile
)

(fn `UserConstructionScript`)