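; BP_IceShard is an ice projectile in the tower defense game that damages and slows enemies.
; When its capsule overlaps an enemy component tagged "Enemy", it applies damage credited to PlayerRef, spawns an ice hit effect and destroys itself.
; Each hit divides the enemy's current max walk speed, so slows stack and nothing here restores them.
; A timer started on BeginPlay destroys shards after a few seconds.
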(event `self.Capsule.OnComponentBeginOverlap`
  (params (OverlappedComponent :type "PrimitiveComponent Object Reference") (OtherActor :type "Actor Object Reference") (OtherComp :type "PrimitiveComponent Object Reference") (OtherBodyIndex :type Integer) (bFromSweep :type Boolean) (SweepResult :type "HitResult Structure (by ref)"))
  (bind _asbp_enemy (cast `/Game/TowerDefense/TD_Blueprints/Enemies/BP_Enemy` OtherActor))
  (if (`ActorComponent.ComponentHasTag` OtherComp "Enemy")
    (`GameplayStatics.ApplyDamage` _asbp_enemy 40.0 (`self.Player Ref`) self "/Script/Engine.DamageType")
    (bind _charactermovement (`Character.CharacterMovement` _asbp_enemy))
    (set `CharacterMovementComponent.MaxWalkSpeed` (/ (`MovementComponent.GetMaxSpeed` _charactermovement) 1.15) _charactermovement)
    (`NiagaraFunctionLibrary.SpawnSystemAtLocation` "/Game/Stylized_VFX_StPack/Particles/UPDATE_1_2/P_Ice_Hit_01.P_Ice_Hit_01" (`self.K2_GetActorLocation`))
    (`self.K2_DestroyActor`)))

(event `self.ReceiveBeginPlay`
  (`KismetSystemLibrary.Delay` 4.0)
  (`self.K2_DestroyActor`) ; Then destroy this projectile
)

(fn `UserConstructionScript`)