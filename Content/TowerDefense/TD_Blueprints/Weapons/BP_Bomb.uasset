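; BP_Bomb is a timed explosive weapon for the tower defense game that detonates three seconds after BeginPlay.
; Detonation spawns an explosion effect and applies radial damage around the actor, ignoring all BP_Tower actors and crediting PlayerRef as causer.
; The explosion sound plays at the world origin rather than at the bomb.
; It then sets the mesh's hidden-in-game flag to false and destroys itself after a short delay.
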(event `self.ReceiveBeginPlay`
  (bind _returnvalue (`self.K2_GetActorLocation`))
  (`KismetSystemLibrary.Delay` 3.0)
  (`NiagaraFunctionLibrary.SpawnSystemAtLocation` "/Game/Stylized_VFX_StPack/VR/VR_Particles/P_VR_ExplosionEffect_02.P_VR_ExplosionEffect_02" _returnvalue)
  (`GameplayStatics.PlaySoundAtLocation` "/Game/FPWeapon/Audio/FirstPersonTemplateWeaponFire02.FirstPersonTemplateWeaponFire02" (0.0 0.0 0.0) (struct) 0.1 1.0 0.0 null null null null)
  (bind _outactors (`GameplayStatics.GetAllActorsOfClass` "/Game/TowerDefense/TD_Blueprints/Towers/BP_Tower.BP_Tower_C"))
  (`GameplayStatics.ApplyRadialDamage` 30.0 _returnvalue 600.0 "/Script/Engine.DamageType" _outactors (`self.PlayerRef`) null)
  (`SceneComponent.SetHiddenInGame` (`self.StaticMesh`) false false)
  (`KismetSystemLibrary.Delay` 1.0)
  (`self.K2_DestroyActor`))

(fn `UserConstructionScript`)