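; Tower defense tower that fires projectiles at the player character.
; When the player overlaps its Box, a looping one-second timer starts calling Shoot.
; Shoot spawns a Bp_Projectile at SpawnProj and pushes its Sphere toward the player's current position with an impulse.
; End overlap clears the Timer handle before pausing it, so the pause misses the running timer and firing continues.
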(event `self.Box.OnComponentBeginOverlap`
  (params (OverlappedComponent :type "PrimitiveComponent Object Reference") (OtherActor :type "Actor Object Reference") (OtherComp :type "PrimitiveComponent Object Reference") (OtherBodyIndex :type Integer) (bFromSweep :type Boolean) (SweepResult :type "HitResult Structure (by ref)"))
  ;[0 0 0] With Collision
  (if (== OtherActor (`GameplayStatics.GetPlayerCharacter` 0))
    (bind _returnvalue (`KismetSystemLibrary.K2_SetTimerDelegate` (delegate `Shoot`) 1.0 true))
    (set `self.Timer` _returnvalue)))

(event `Shoot`
  ;[0 0 0] With Collision
  (bind _returnvalue (`|SpawnActorFromClass` "/Game/TowerDefense/TD_Blueprints/Bp_Fabien/Bp_Projectile.Bp_Projectile_C" (`SceneComponent.K2_GetComponentToWorld` (`self.SpawnProj`)) "Undefined" "MultiplyWithRoot" null null))
  (`PrimitiveComponent.AddImpulse` (`/Game/TowerDefense/TD_Blueprints/Bp_Fabien/Bp_Projectile.Sphere` _returnvalue) (* (`KismetMathLibrary.GetDirectionUnitVector` (`self.K2_GetActorLocation` _returnvalue) (`self.K2_GetActorLocation` (`GameplayStatics.GetPlayerCharacter` 0))) 5000.0) "None" false))

(event `self.Box.OnComponentEndOverlap`
  (params (OverlappedComponent :type "PrimitiveComponent Object Reference") (OtherActor :type "Actor Object Reference") (OtherComp :type "PrimitiveComponent Object Reference") (OtherBodyIndex :type Integer))
  ;[0 0 0] With Collision
  (if (== OtherActor (`GameplayStatics.GetPlayerCharacter` 0))
    (bind _output_get (set `self.Timer` (struct)))
    (`KismetSystemLibrary.K2_PauseTimerHandle` _output_get)))

(fn `UserConstructionScript`)