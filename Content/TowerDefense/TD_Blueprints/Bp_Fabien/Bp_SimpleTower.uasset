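; Tower defense tower that fires projectiles at enemies inside its collision range and passes damage taken to its parent's life update.
; Overlap events maintain a list of tagged enemies and start looping timers on each entry.
; A fast timer prunes dead enemies and picks a target when none is valid.
; A slower one launches projectiles by impulse toward it, pausing when the target is dead or invalid.
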(event `self.ReceiveBeginPlay`
  ;[0 0 0] Set health
  (`parent.ReceiveBeginPlay`)
  (set `self.Health` 300.0))

(event `Shoot`
  ;[0 0 0] Shoot system
  (bind _target (`self.Target`)
    (:`then`
      (if (`/Game/TowerDefense/TD_Blueprints/Enemies/BP_Enemy.IsDead` _target)
        (`KismetSystemLibrary.K2_PauseTimerHandle` (`self.TimerShoot`))
        (else
          (bind _returnvalue (`|SpawnActorFromClass` "/Game/TowerDefense/TD_Blueprints/Bp_Fabien/Bp_Projectile.Bp_Projectile_C" (`SceneComponent.K2_GetComponentToWorld` (`self.SpawnProj`)) "Undefined" "MultiplyWithRoot" null null))
          (`PrimitiveComponent.AddImpulse` (`/Game/TowerDefense/TD_Blueprints/Bp_Fabien/Bp_Projectile.Sphere` _returnvalue) (* (`KismetMathLibrary.GetDirectionUnitVector` (`self.K2_GetActorLocation` _returnvalue) (`self.K2_GetActorLocation` _target)) 10000.0) "None" false))))
    (:`else`
      (`KismetSystemLibrary.K2_PauseTimerHandle` (`self.TimerShoot`)))))

(event `Check Target`
  ;[0 0 0] Verify if the array is empty or not
  (if (not (`KismetArrayLibrary.Array_IsEmpty` (`self.Enemies in range`)))
    ;[0 0 0] Set new target
    (for _array_element (`self.Enemies in range`)
      (if (`/Game/TowerDefense/TD_Blueprints/Enemies/BP_Enemy.IsDead` _array_element)
        (`KismetArrayLibrary.Array_RemoveItem` (`self.Enemies in range`))
        (else
          (`self.Target`
            (:`then`)
            (:`else`
              (set `self.Target` _array_element))))))))

(event `self.Collision.OnComponentBeginOverlap`
  (params (OverlappedComponent :type "PrimitiveComponent Object Reference") (OtherActor :type "Actor Object Reference") (OtherComp :type "PrimitiveComponent Object Reference") (OtherBodyIndex :type Integer) (bFromSweep :type Boolean) (SweepResult :type "HitResult Structure (by ref)"))
  ;[0 0 0] Detect enemy in range
  (if (`self.ActorHasTag` OtherActor "Enemy")
    (bind _asbp_enemy (cast `/Game/TowerDefense/TD_Blueprints/Enemies/BP_Enemy` OtherActor))
    (`KismetArrayLibrary.Array_AddUnique` (`self.Enemies in range`) _asbp_enemy)
    (`KismetSystemLibrary.K2_SetTimerDelegate` (delegate `Check Target`) 0.1 true)
    (bind _returnvalue (`KismetSystemLibrary.K2_SetTimerDelegate` (delegate `Shoot`) 1.0 true))
    (set `self.TimerShoot` _returnvalue)))

(event `self.Collision.OnComponentEndOverlap`
  (params (OverlappedComponent :type "PrimitiveComponent Object Reference") (OtherActor :type "Actor Object Reference") (OtherComp :type "PrimitiveComponent Object Reference") (OtherBodyIndex :type Integer))
  ;[0 0 0] Remove enemy when out of range
  (if (`self.ActorHasTag` OtherActor "Enemy")
    (bind _asbp_enemy (cast `/Game/TowerDefense/TD_Blueprints/Enemies/BP_Enemy` OtherActor))
    (`KismetArrayLibrary.Array_RemoveItem` (`self.Enemies in range`) _asbp_enemy)))

(event `self.ReceiveAnyDamage`
  (params (Damage :type "Float (single-precision)") (DamageType :type "DamageType Object Reference") (InstigatedBy :type "Controller Object Reference") (DamageCauser :type "Actor Object Reference"))
  ;[0 0 0] Update life
  (`self.UpdateLife` Damage))

(fn `UpdateLife`
  (params (Damage :type "Float (double-precision)"))
  (`parent.UpdateLife` Damage))

(fn `UserConstructionScript`)