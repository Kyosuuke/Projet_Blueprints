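; Mortar Blueprint for a tower defense game that spawns an actor, presumably its shell, after the player enters its trigger box.
; Box begin overlap with player 0's character starts a five-second one-shot timer, which fires ShootBullet to spawn at the SpawnBullet component's transform.
; End overlap does nothing, as the logic to clear and pause the timer is disconnected, so leaving the box does not cancel the shot.
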(event `self.Box.OnComponentBeginOverlap`
  (params (OverlappedComponent :type "PrimitiveComponent Object Reference") (OtherActor :type "Actor Object Reference") (OtherComp :type "PrimitiveComponent Object Reference") (OtherBodyIndex :type Integer) (bFromSweep :type Boolean) (SweepResult :type "HitResult Structure (by ref)"))
  (if (== OtherActor (`GameplayStatics.GetPlayerCharacter` 0))
    (`KismetSystemLibrary.K2_SetTimerDelegate` (delegate `Shoot bullet`) 5.0)))

(event `Shoot bullet`
  (`|SpawnActorFromClass` "/Game/TowerDefense/TD_Blueprints/Bp_Fabien/Bp_Bullet.Bp_Bullet_C" (`SceneComponent.K2_GetComponentToWorld` (`self.SpawnBullet`)) "Undefined" "MultiplyWithRoot" null null))

(event `self.Box.OnComponentEndOverlap`
  (params (OverlappedComponent :type "PrimitiveComponent Object Reference") (OtherActor :type "Actor Object Reference") (OtherComp :type "PrimitiveComponent Object Reference") (OtherBodyIndex :type Integer)))

(fn `UserConstructionScript`)