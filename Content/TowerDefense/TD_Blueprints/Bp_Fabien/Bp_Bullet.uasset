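; Tower defense bullet actor that explodes on enemy hits and deals area damage.
; Its capsule overlap continues only for BP_Enemy actors, then checks the overlapped component for the "Enemy" tag.
; A tagged hit spawns an energy explosion effect, applies radial damage around the bullet and destroys it.
; An untagged enemy component destroys the bullet after a short delay, while overlaps with other actors are ignored.
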(event `self.Capsule.OnComponentBeginOverlap`
  (params (OverlappedComponent :type "PrimitiveComponent Object Reference") (OtherActor :type "Actor Object Reference") (OtherComp :type "PrimitiveComponent Object Reference") (OtherBodyIndex :type Integer) (bFromSweep :type Boolean) (SweepResult :type "HitResult Structure (by ref)"))
  ;[0 0 0] Detect and apply damage if is an enemy
  (cast `/Game/TowerDefense/TD_Blueprints/Enemies/BP_Enemy` OtherActor)
  (if (`ActorComponent.ComponentHasTag` OtherComp "Enemy")
    (`NiagaraFunctionLibrary.SpawnSystemAtLocation` "/Game/Stylized_VFX_StPack/Particles/P_ExplosionEnergy_02.P_ExplosionEnergy_02" (`self.K2_GetActorLocation`) (struct) (10.0 10.0 10.0))
    (`GameplayStatics.ApplyRadialDamage` :`BaseDamage` (`self.Damage`) :`Origin` (`self.K2_GetActorLocation`) :`DamageRadius` 500.0 :`DamageCauser` self :`InstigatedByController` null)
    (`self.K2_DestroyActor`)
    (else
      (`KismetSystemLibrary.Delay` 1.5)
      (`self.K2_DestroyActor`))))

(fn `UserConstructionScript`)