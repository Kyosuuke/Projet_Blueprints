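; BP_BulletBill is a tower defense actor that homes in on the BPSpawnDemo actor it finds at BeginPlay and treats as the tower.
; Each tick it moves toward that tower at Speed, scaled by delta time, and rotates to face it.
; Its Box overlap stops movement on contact with the tower and restores a fixed speed when contact ends.
; Disconnected logic would tint a Niagara effect by player distance, but never runs.
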(event `self.ReceiveBeginPlay`
  (bind _returnvalue (`GameplayStatics.GetActorOfClass` "/Game/Blueprints/BPSpawnDemo.BPSpawnDemo_C"))
  (set `self.Tower` _returnvalue))

(event `self.ReceiveTick`
  (params (DeltaSeconds :type "Float (single-precision)"))
  (bind _returnvalue (`KismetMathLibrary.Normal` (- (`self.K2_GetActorLocation` (`self.Tower`)) (`self.K2_GetActorLocation`))))
  (`SceneComponent.K2_SetWorldLocationAndRotation` (`self.DefaultSceneRoot`) (+ (* DeltaSeconds (`self.speed`) _returnvalue) (`self.K2_GetActorLocation`)) (`KismetMathLibrary.MakeRotFromX` _returnvalue) false false))

(event `self.Box.OnComponentBeginOverlap`
  (params (OverlappedComponent :type "PrimitiveComponent Object Reference") (OtherActor :type "Actor Object Reference") (OtherComp :type "PrimitiveComponent Object Reference") (OtherBodyIndex :type Integer) (bFromSweep :type Boolean) (SweepResult :type "HitResult Structure (by ref)"))
  (if (== OtherActor (`self.Tower`))
    (set `self.speed` 0.0)))

(event `self.Box.OnComponentEndOverlap`
  (params (OverlappedComponent :type "PrimitiveComponent Object Reference") (OtherActor :type "Actor Object Reference") (OtherComp :type "PrimitiveComponent Object Reference") (OtherBodyIndex :type Integer))
  (if (== OtherActor (`self.Tower`))
    (set `self.speed` 500.0)))

(fn `UserConstructionScript`)